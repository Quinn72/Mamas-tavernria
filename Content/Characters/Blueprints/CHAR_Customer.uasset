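; Customer character that walks between tagged waypoints and can be interacted with by the first-person player.
; On BeginPlay it AI-moves to the WaypointSet1 actor at its ID index, then after a short delay to the matching WaypointSet2 actor.
; Interaction from a first-person controller sets ItemString to a random String array entry, with the random index bounded by the Items array's length.
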(event EventBeginPlay
  (Utilities|FlowControl|Sequence
    (:then_0
      (bind _outactors (Actor|GetAllActorswithTag "WaypointSet1"))
      (bind _output_get (Variables|Default|SetWaypoints _outactors))
      (Utilities|FlowControl|DelayUntilNextTick)
      (AI|AIMoveTo self "0, 0, 0" (Utilities|Array|Get(acopy) _output_get (Variables|Default|GetID)) 5.0 false
        (:OnSuccess
          (bind _outactors_2 (Actor|GetAllActorswithTag "WaypointSet2"))
          (bind _output_get_2 (Variables|Default|SetWaypoints _outactors_2))
          (Utilities|FlowControl|Delay 5.0)
          (AI|AIMoveTo self "0, 0, 0" (Utilities|Array|Get(acopy) _output_get_2 (Variables|Default|GetID)) 5.0 false))))
    (:then_1
      (Variables|Default|SetMEME 0))))

(event EventOnInteract
  (params (Character%20 :type BP%20First%20Person%20Character%20Object%20Reference))
  (Utilities|Casting|CastToPC_FirstPerson (Pawn|GetController Character%20))
  (Variables|Default|SetItem%20string%20 (Utilities|Array|Get(acopy) (Variables|Default|GetString) (Math|Random|RandomInteger (Utilities|Array|Length (Variables|Default|GetItems))))))

(fn ConstructionScript)

(fn IsInteractable
  (return true))