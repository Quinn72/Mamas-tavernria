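; BP_Paper is a paper actor that records which ink and monster stamp have been applied to it through collisions.
; Its Hit event reads actor tags in stages: blue, black or red ink first, then a dragon, goblin or undead stamp.
; Each stage sets one exclusive choice flag and a completion flag that opens the next.
; The final chest stage checks gold, weapon, spell and potion tags but sets nothing yet.
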(event Collision|EventHit
  (params (MyComp :type Primitive%20Component%20Object%20Reference) (Other :type Actor%20Object%20Reference) (OtherComp :type Primitive%20Component%20Object%20Reference) (bSelfMoved :type Boolean) (HitLocation :type Vector :default "0, 0, 0") (HitNormal :type Vector :default "0, 0, 0") (NormalImpulse :type Vector :default "0, 0, 0") (Hit :type Hit%20Result%20Structure%20%28by%20ref%29))
  (if (Variables|Default|GetbHasInk)
    (if (Variables|Default|GetbHasMonster)
      (if (not (Variables|Default|GetbHasChest))
        (if (not (Actor|ActorHasTag Other "ChestGold"))
          (if (not (Actor|ActorHasTag Other "ChestWeapon"))
            (if (not (Actor|ActorHasTag Other "ChestSpell"))
              (if (Actor|ActorHasTag Other "ChestPotion")
                _)))))
      (elif (Actor|ActorHasTag Other "StampDragon")
        (Variables|Default|SetbHadDragon true)
        (Variables|Default|SetbHasGoblin false)
        (Variables|Default|SetbHasUndead false)
        (if (Math|Boolean|ORBoolean (Variables|Default|GetbHadDragon) (Variables|Default|GetbHasGoblin) (Variables|Default|GetbHasUndead)) :!label _label
          (Variables|Default|SetbHasMonster true))
        (elif (Actor|ActorHasTag Other "StampGoblin")
          (Variables|Default|SetbHasGoblin true)
          (Variables|Default|SetbHadDragon false)
          (Variables|Default|SetbHasUndead false)
          (goto _label)
          (elif (Actor|ActorHasTag Other "StampUndead")
            (Variables|Default|SetbHasUndead true)
            (Variables|Default|SetbHadDragon false)
            (Variables|Default|SetbHasGoblin false)
            (goto _label)))))
    (elif (Actor|ActorHasTag Other "BlueInk")
      (Variables|Default|SetbHasBlueInk true)
      (Variables|Default|SetbHasBlackInk false)
      (Variables|Default|SetbHasRedInk false)
      (if (Math|Boolean|ORBoolean (Variables|Default|GetbHasBlueInk) (Variables|Default|GetbHasBlackInk) (Variables|Default|GetbHasRedInk)) :!label _label_2
        (Variables|Default|SetbHasInk true))
      (elif (Actor|ActorHasTag Other "BlackInk")
        (Variables|Default|SetbHasBlackInk true)
        (Variables|Default|SetbHasBlueInk false)
        (Variables|Default|SetbHasRedInk false)
        (goto _label_2)
        (elif (Actor|ActorHasTag Other "RedInk")
          (Variables|Default|SetbHasRedInk true)
          (Variables|Default|SetbHasBlueInk false)
          (Variables|Default|SetbHasBlackInk false)
          (goto _label_2))))))

(fn ConstructionScript)